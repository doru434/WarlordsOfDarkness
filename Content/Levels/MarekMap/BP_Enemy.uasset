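; BP_Enemy is an enemy actor whose static mesh slides back and forth along its relative X axis.
; On BeginPlay it stores the start location and an end point 150 units away, then a timeline lerps the mesh between them without sweeping.
; The timeline's Update pin, rather than Finished, feeds a Delay that toggles the Loop flag to alternate Play and Reverse.
; The file contains no AI, damage or collision logic.
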(event `self.ReceiveBeginPlay`
  (bind _returnvalue_location (`KismetMathLibrary.BreakTransform` (`SceneComponent.GetRelativeTransform` (`self.StaticMeshComponent`))))
  (set `self.StartLoc` (`SceneComponent.RelativeLocation` (`self.StaticMeshComponent`)))
  (set `self.EndLoc` (+ _returnvalue_location (150.0 0.0 0.0)))
  (bind (_direction _newtrack_2) (`Timeline|Timeline_0` :!label _label)
    (:`Update`
      (`SceneComponent.K2_SetRelativeLocation` (`self.StaticMeshComponent`) (`KismetMathLibrary.VLerp` (`self.StartLoc`) (`self.EndLoc`) _newtrack_2) false false)
      (`KismetSystemLibrary.Delay` (`self.Delay`))
      (if (`self.Loop`)
        (set `self.Loop` false)
        (goto _label :!via `Reverse`)
        (else
          (set `self.Loop` true)
          (goto _label))))))

(fn `UserConstructionScript`)