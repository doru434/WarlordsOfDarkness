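; BP_WorldSegment is a world map segment actor that can be selected and unselected, using a Plane component as its highlight.
; On BeginPlay it binds to the CorePlayerController's selection delegate.
; SelectActor fires that delegate, then either unselects an already selected segment or shows the Plane and adds itself to the WOD player pawn's SelectedActors.
; UnselectActor hides the Plane and removes the segment from that array.
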(event `self.ReceiveBeginPlay`
  (bind _ascore_player_controller (cast `CorePlayerController` (`GameplayStatics.GetPlayerController` 0)))
  (add `CorePlayerController.OnSelectionDelegate` _ascore_player_controller (`|CreateDelegate` :!event `UnselectActor`)))

(event `self.SelectActor`
  (bind _playerpawn (`/Game/Core/BP_FunctionLibrary.GetWODPlayerPawn`))
  (bind _ascore_player_controller (cast `CorePlayerController` (`GameplayStatics.GetPlayerController` 0)))
  (`CorePlayerController.OnSelectionDelegate` _ascore_player_controller)
  (if (`self.Selected`)
    (`self.UnselectActor`)
    (else
      (`SceneComponent.SetVisibility` (`self.Plane`) true false)
      (set `self.Selected` true)
      (`/Engine/EditorBlueprintResources/StandardMacros.IsValid` _playerpawn
        (:`Is Valid`
          (`KismetArrayLibrary.Array_Add` (`PlayerPawn.SelectedActors` _playerpawn) self)
          (cast `/Game/Core/GM_WorldMap` (`GameplayStatics.GetGameMode`)))))))

(event `self.UnselectActor`
  (bind _playerpawn (`/Game/Core/BP_FunctionLibrary.GetWODPlayerPawn`))
  (bind _selectedactors (`PlayerPawn.SelectedActors` _playerpawn))
  (bind _returnvalue (`KismetArrayLibrary.Array_Find` _selectedactors self))
  (`SceneComponent.SetVisibility` (`self.Plane`) false false)
  (set `self.Selected` false)
  (`/Engine/EditorBlueprintResources/StandardMacros.IsValid` _playerpawn
    (:`Is Valid`
      (if (!= _returnvalue -1)
        (`KismetArrayLibrary.Array_Remove` _selectedactors _returnvalue)))))

(fn `UserConstructionScript`)