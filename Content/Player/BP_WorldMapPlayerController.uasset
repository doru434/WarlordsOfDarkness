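; Player controller for the world map that handles mouse selection of actors.
; A selection click traces under the cursor, sends a select message to the hit actor and passes its display name to the world map widget via the game mode as the mission name.
; BeginPlay sets a very long hit result trace distance for the cursor traces.
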(event `InputAction|MouseSelection`
  (params (Key :type "Key Structure"))
  (:`Pressed`
    (bind _returnvalue (`self.GetTraceUnderCursor` "TraceTypeQuery3"))
    (bind (_bblockinghit _binitialoverlap _time _distance _location _impactpoint _normal _impactnormal _physmat _hitactor) (`GameplayStatics.BreakHitResult` _returnvalue))
    (if _bblockinghit
      (message `SelectionInterface.SelectActor` _hitactor)
      (bind _asgm_world_map (cast `/Game/Core/GM_WorldMap` (`GameplayStatics.GetGameMode`)))
      (`/Game/Levels/WorldMap/UI/WB_WorldMap.UpdateMissionName` (`/Game/Core/GM_WorldMap.WidgetWorldMap` _asgm_world_map) (`KismetTextLibrary.Conv_StringToText` (`KismetSystemLibrary.GetDisplayName` _hitactor))))))

(event `self.ReceiveBeginPlay`
  (`parent.ReceiveBeginPlay`)
  (set `self.HitResultTraceDistance` 1000000.0))

(fn `UserConstructionScript`
  (`parent.UserConstructionScript`))