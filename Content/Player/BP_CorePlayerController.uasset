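; BP_CorePlayerController is the player controller that handles RTS-style mouse selection and move orders for friendly characters.
; Pressing MouseSelection flags selection active, unselects the pawn's SelectedActors through SelectionInterface and passes the starting mouse position to HUD_RTS.
; Releasing it clears the flag, which is exposed through a getter.
; MouseAction tells selected BP_BaseCharacterFriendly actors on the WOD player pawn to move to the mouse position.
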(event `InputAction|MouseSelection`
  (params (Key :type "Key Structure"))
  (:`Pressed`
    (`self.DeselectPreviousSelection`)
    (`self.UpdateHUDStartingMousePosition`))
  (:`Released`
    (set `self.IsSelectionActive` false)))

(event `self.ReceiveTick`
  (params (DeltaSeconds :type "Float (single-precision)")))

(event `InputAction|MouseAction`
  (params (Key :type "Key Structure"))
  (bind _playerpawn (`/Game/Core/BP_FunctionLibrary.GetWODPlayerPawn`))
  (:`Pressed`
    (`/Engine/EditorBlueprintResources/StandardMacros.IsValid` _playerpawn
      (:`Is Valid`
        (for _array_element (`PlayerPawn.SelectedActors` _playerpawn)
          (bind _asbp_base_character_friendly (cast `/Game/Characters/BP_BaseCharacterFriendly` _array_element))
          (`/Game/Characters/BP_BaseCharacterFriendly.MoveToMousePosition` _asbp_base_character_friendly))))))

(fn `DeselectPreviousSelection`
  (set `self.IsSelectionActive` true)
  (for _array_element (`PlayerPawn.SelectedActors` (`/Game/Core/BP_FunctionLibrary.GetWODPlayerPawn`))
    (bind _asselection_interface (cast `SelectionInterface` _array_element))
    (`SelectionInterface.UnselectActor` _asselection_interface)))

(fn `Get Selection Active`
  (returns (SelectionActive :type Boolean))
  (return (`self.IsSelectionActive`)))

(fn `UpdateHUDStartingMousePosition`
  (bind (_locationx _locationy) (`self.GetMousePosition` (`GameplayStatics.GetPlayerController` 0)))
  (bind _ashud_rts (cast `/Game/Modules/Selection/HUD_RTS` (`self.GetHUD`)))
  (set `/Game/Modules/Selection/HUD_RTS.StartingMousePosition` (`KismetMathLibrary.MakeVector2D` _locationx _locationy) _ashud_rts))

(fn `UserConstructionScript`)