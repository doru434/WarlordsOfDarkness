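; Base character for selectable units, handling team decal, move orders, damage and death, with a display widget created per unit.
; Move orders trace under the cursor and write the hit location to the AI controller's Blackboard Destination key.
; Damage reduces Health; death ragdolls the mesh, detaches the controller, unregisters perception stimuli and destroys the actor after a delay.
; Tick resets the Casted flag once its cooldown elapses.
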(event `self.ReceiveTick`
  (params (DeltaSeconds :type "Float (single-precision)"))
  (if (`self.Casted`)
    (bind _output_get (set `self.ElapsedTime` (+ DeltaSeconds (`self.ElapsedTime`))))
    (if (>= _output_get (`self.Cooldown`))
      (set `self.Casted` false)
      (set `self.ElapsedTime` 0.0))))

(event `DestroyCharacterAfterTime`
  (params (Time :type "Float (double-precision)"))
  (`KismetSystemLibrary.Delay` Time)
  (`self.K2_DestroyActor`))

(event `self.ReceiveBeginPlay`
  (bind _returnvalue (`|CreateWidget` "/Game/UnitSkills/UI/Display_UI.Display_UI_C"))
  (bind _output_get (set `self.DisplayUnitUI` _returnvalue))
  (`UserWidget.AddToViewport` _output_get 0)
  (switch `EFriendOrFoe` (`self.E_FriendOrFoe`)
    (:`Friend`
      (`DecalComponent.SetDecalMaterial` (`self.SelectionDecalComponent`) "/Game/Materials/MI_DecalRingFriendly.MI_DecalRingFriendly"))
    (:`Foe`
      (`DecalComponent.SetDecalMaterial` (`self.SelectionDecalComponent`) "/Game/Materials/MI_DecalRingEnemy.MI_DecalRingEnemy"))))

(event `MoveToMousePosition`
  (bind (_hitresult _returnvalue) (`PlayerController.GetHitResultUnderCursorByChannel` (`GameplayStatics.GetPlayerController` 0) "TraceTypeQuery4" true))
  (if _returnvalue
    (`/Engine/EditorBlueprintResources/StandardMacros.IsValid` self
      (:`Is Valid`
        (`BlackboardComponent.SetValueAsVector` (`AIBlueprintHelperLibrary.GetBlackboard` (`AIBlueprintHelperLibrary.GetAIController` self)) (`self.Destination`) (`.Location` (`GameplayStatics.BreakHitResult` _hitresult)))))))

(event `self.ReceiveDamage`
  (params (Damage :type "Float (single-precision)"))
  ;[1 0.3038 0.3038] Damage Interface
  (bind _output_get (set `self.Health` (- (`self.Health`) Damage)))
  (if (<= _output_get 0.0)
    (`self.Die`)
    (`self.DestroyCharacterAfterTime` 2.0)))

(event `self.InflictDamage`
  (params (Damage :type "Float (single-precision)") (ActorToDamage :type "Actor Object Reference"))
  ;[1 0.3038 0.3038] Damage Interface
  (message `DamageInterface.ReceiveDamage` ActorToDamage Damage))

(event `self.Die`
  (bind _aiperceptionstimulisource (`self.AIPerceptionStimuliSource`))
  ;[1 0.3038 0.3038] Damage Interface
  (`PrimitiveComponent.SetSimulatePhysics` (`self.Mesh`) true)
  (`CharacterMovementComponent.DisableMovement` (`self.CharacterMovement`))
  (`self.DetachFromControllerPendingDestroy`)
  (`AIPerceptionStimuliSourceComponent.UnregisterFromPerceptionSystem` _aiperceptionstimulisource)
  (`AIPerceptionStimuliSourceComponent.UnregisterFromSense` _aiperceptionstimulisource "/Script/AIModule.AISense_Sight"))

(fn `UserConstructionScript`)