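; BP_EnemyDetourAiController is an enemy AI controller that runs the BT_BaseEnemy behavior tree on BeginPlay.
; When AI perception successfully senses an actor, it stores that actor as the Blackboard Target, but only if no valid target is already set.
; It never clears the target on lost perception, and prints each target perception update for debugging.
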(event `self.ReceiveBeginPlay`
  (`parent.ReceiveBeginPlay`)
  (`self.RunBehaviorTree` "/Game/Characters/AI/Enemy/BT_BaseEnemy.BT_BaseEnemy"))

(event `self.AIPerception.OnTargetPerceptionUpdated`
  (params (Actor :type "Actor Object Reference") (Stimulus :type "AIStimulus Structure"))
  (bind _blackboard (`self.Blackboard`))
  (`KismetSystemLibrary.PrintString` (`KismetStringLibrary.Concat_StrStr` "PerceptionUpdated by: " (`KismetSystemLibrary.GetDisplayName` Actor)) true true (struct :`G` 0.66 :`B` 1.0 :`A` 1.0) 1.0)
  (`/Engine/EditorBlueprintResources/StandardMacros.IsValid` _blackboard
    (:`Is Valid`
      (if (`.bSuccessfullySensed` (break `AIStimulus` Stimulus))
        (`/Engine/EditorBlueprintResources/StandardMacros.IsValid` (`BlackboardComponent.GetValueAsObject` _blackboard (`self.Target`))
          (:`Is Not Valid`
            (`BlackboardComponent.SetValueAsObject` _blackboard (`self.Target`) Actor)))))))

(event `self.AIPerception.OnTargetPerceptionInfoUpdated`
  (params (UpdateInfo :type "ActorPerceptionUpdateInfo Structure (by ref)")))

(event `self.AIPerception.OnPerceptionUpdated`
  (params (UpdatedActors :type "Array of Actor Object Reference (by ref)")))

(fn `UserConstructionScript`
  (`parent.UserConstructionScript`))