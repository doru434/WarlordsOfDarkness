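; Patrol point actor that acts as an editable waypoint for the BP_BaseCharacterEnemy referenced in ActorAttached.
; It holds no path logic and forwards its events to that enemy through a cast.
; Its construction script has the enemy redraw the debug path, and its Destroyed event reports the removed point through OnPointDestroyedInEditor.
; CreatePatrolPoint passes requests for new points on to the enemy.
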(event `self.ReceiveBeginPlay`)

(event `self.ReceiveDestroyed`
  (bind _asbp_base_character_enemy (cast `/Game/Characters/BP_BaseCharacterEnemy` (`self.ActorAttached`)))
  (`/Game/Characters/BP_BaseCharacterEnemy.OnPointDestroyedInEditor` _asbp_base_character_enemy self))

(fn `CreatePatrolPoint`
  (bind _asbp_base_character_enemy (cast `/Game/Characters/BP_BaseCharacterEnemy` (`self.ActorAttached`)))
  (`/Game/Characters/BP_BaseCharacterEnemy.CreatePatrolPoint` _asbp_base_character_enemy))

(fn `UserConstructionScript`
  (bind _asbp_base_character_enemy (cast `/Game/Characters/BP_BaseCharacterEnemy` (`self.ActorAttached`)))
  (`/Game/Characters/BP_BaseCharacterEnemy.DrawDebugPath` _asbp_base_character_enemy))